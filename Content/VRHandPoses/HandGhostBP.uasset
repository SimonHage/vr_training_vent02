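; HandGhostBP is a ghost hand actor that previews VR grab poses on a mannequin hand mesh.
; UpdatePose, also called from the Construction Script, passes the grip state and specific grab type to MannequinHand_Right_AnimBP.
; A Gate lets it enable the AnimBP's debug force-grab override until BeginPlay clears that flag and closes the gate.
; Disconnected test logic, including a timed grab-type cycle, remains in the graph.
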(event `self.ReceiveBeginPlay`
  (bind _asmannequin_hand_right_anim_bp (cast `/Game/VRHandPoses/UnrealVRHand/Mesh/MannequinHand_Right_AnimBP` (`SkeletalMeshComponent.GetAnimInstance` (`self.HandMesh`))))
  (set `/Game/VRHandPoses/UnrealVRHand/Mesh/MannequinHand_Right_AnimBP.CurGrabDebugOverwrite-ForceGrabInEditor` false _asmannequin_hand_right_anim_bp)
  (goto _label :!via `Close`))

(event `UpdatePose`
  ;[1 1 1] Also fires through construction script
  (bind _asmannequin_hand_right_anim_bp (cast `/Game/VRHandPoses/UnrealVRHand/Mesh/MannequinHand_Right_AnimBP` (`SkeletalMeshComponent.GetAnimInstance` (`self.HandMesh`))))
  (`/Game/VRHandPoses/UnrealVRHand/Mesh/MannequinHand_Right_AnimBP.SetPose` _asmannequin_hand_right_anim_bp (`self.GripState`) (`self.CurSpecificGrabType`) true false)
  (`/Engine/EditorBlueprintResources/StandardMacros.Gate` false :!label _label
    (:`Exit`
      (set `/Game/VRHandPoses/UnrealVRHand/Mesh/MannequinHand_Right_AnimBP.CurGrabDebugOverwrite-ForceGrabInEditor` true _asmannequin_hand_right_anim_bp))))

(fn `UserConstructionScript`
  (`self.UpdatePose`))