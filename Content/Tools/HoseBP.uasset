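; Hose actor that renders a physics-simulated Cable component as a chain of spline meshes with the hose material.
; While Update is set, Tick rebuilds segments from cable particle locations, with a configurable skip, reusing existing meshes.
; Tangents follow neighbouring particles and align to both end components' forward vectors, whose directions also drive the cable force.
; An event reattaches the free end to another component and sets cable length.
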(event `SetAttachEndToComponent`
  (params (Component :type "SceneComponent Object Reference") (Length :type "Float (double-precision)" :default 100.0))
  (bind _cable (`self.Cable`))
  (set `self.CurAttachEndCompoent` Component)
  (`CableComponent.SetAttachEndToComponent` _cable Component "None")
  (set `CableComponent.CableLength` Length _cable))

(event `self.ReceiveBeginPlay`
  (`self.Regenerate`))

(event `Regenerate`
  (bind _defaultattachendtocomponent (`self.DefaultAttachEndToComponent`))
  (bind _allsplinemeshes (`self.AllSplineMeshes`))
  (`ActorComponent.K2_DestroyComponent` _allsplinemeshes)
  (`KismetArrayLibrary.Array_Clear` _allsplinemeshes)
  (`CableComponent.SetAttachEndToComponent` (`self.Cable`) _defaultattachendtocomponent "None")
  (set `self.CurAttachEndCompoent` _defaultattachendtocomponent)
  (goto _label :!via `Open`))

(event `self.ReceiveTick`
  (params (DeltaSeconds :type "Float (single-precision)"))
  (`/Engine/EditorBlueprintResources/StandardMacros.Gate` true :!label _label
    (:`Exit`
      (if (`self.Update`)
        (`self.PopulateCableWithSplineSegments`)))))

(fn `IndexAddWithSplineMeshSkip`
  (params (Index :type Integer) (Add :type Integer) (WithoutSkipInstead :type Boolean) (HalfSkipInstead :type Boolean))
  (returns (NewIndex :type Integer))
  (bind _splinemeshstepsskip (`self.SplineMeshStepsSkip`))
  (bind _cableparticleslastindex (`self.CableParticlesLastIndex`))
  (bind _returnvalue (`KismetMathLibrary.Min` (`KismetMathLibrary.FCeil` (* (+ Index Add) _splinemeshstepsskip)) _cableparticleslastindex))
  (bind _returnvalue_2 (+ (`KismetMathLibrary.Min` (`KismetMathLibrary.FCeil` (* Index _splinemeshstepsskip)) _cableparticleslastindex) Add))
  (return (`KismetMathLibrary.SelectInt` (`KismetMathLibrary.Round` (`KismetMathLibrary.Lerp` (`KismetMathLibrary.Conv_IntToDouble` _returnvalue_2) (`KismetMathLibrary.Conv_IntToDouble` _returnvalue) 0.5)) (`KismetMathLibrary.SelectInt` _returnvalue_2 _returnvalue WithoutSkipInstead) HalfSkipInstead)))

(fn `PopulateCableWithSplineSegments`
  (locals (CurIndex :type Integer :default 0) (AllSplinesMeshesForUpdate :type "Array of SplineMeshComponent Object Reference") (CurSplineMesh :type "SplineMeshComponent Object Reference") (CurNextIndex :type Integer :default 0) (LastEndTangent :type "Vector Structure" :default (0.0 0.0 0.0)) (CurCableFactor :type "Float (double-precision)" :default 0.0) (LastPosition :type "Vector Structure" :default (0.0 0.0 0.0)))
  (bind _returnvalue (`KismetMathLibrary.MakeTransform` (0.0 0.0 0.0)))
  (bind _scalehose (`self.ScaleHose`))
  (bind _tangentlengthfactor (`self.TangentLengthFactor`))
  (bind _allsplinesmeshesforupdate (`local.AllSplinesMeshesForUpdate`))
  (bind _cursplinemesh (`local.CurSplineMesh`))
  (bind _locations (`CableComponent.GetCableParticleLocations` (`self.Cable`)))
  (bind _returnvalue_2 (`KismetArrayLibrary.Array_LastIndex` _locations))
  (bind _returnvalue_3 (`KismetMathLibrary.InverseTransformLocation` (`self.GetTransform`) (`|GetArrayItem` _locations (`local.CurNextIndex`))))
  (bind _returnvalue_4 (+ _returnvalue_3 (0.0 0.0 0.0)))
  (set `CableComponent.CableForce` (+ (* (* (`SceneComponent.GetForwardVector` (`self.DefaultAttachEndToComponent`)) -1.0) (`self.CableEndDirectionForceOnAll`)) (* (* (`SceneComponent.GetForwardVector` (`self.Start`)) -1.0) (`self.CableStartDirectionForceOnAll`))) (`self.Cable`))
  (set `local.AllSplinesMeshesForUpdate` (`self.AllSplineMeshes`))
  (set `self.CableParticlesLastIndex` _returnvalue_2)
  (for _index (range (+ (`KismetMathLibrary.Round` (/ (`KismetMathLibrary.Conv_IntToDouble` _returnvalue_2) (`self.SplineMeshStepsSkip`))) 1))
    (bind _output_get (set `local.CurIndex` (`self.IndexAddWithSplineMeshSkip` _index)))
    (set `local.CurCableFactor` (/ (`KismetMathLibrary.Conv_IntToDouble` _output_get) (`KismetMathLibrary.Conv_IntToDouble` (`self.CableParticlesLastIndex`))))
    (set `local.CurNextIndex` (`self.IndexAddWithSplineMeshSkip` _index 1))
    (if (< _output_get _returnvalue_2)
      (if (`KismetArrayLibrary.Array_IsValidIndex` _allsplinesmeshesforupdate)
        (bind _output_get_2 (set `local.CurSplineMesh` (`|GetArrayItem` _allsplinesmeshesforupdate)))
        (`SceneComponent.K2_SetRelativeTransform` _output_get_2 _returnvalue false false)
        (`KismetArrayLibrary.Array_Remove` _allsplinesmeshesforupdate)
        (else
          (bind _returnvalue_5 (`AddComponent|NODE_AddSplineMeshComponent-0` :`RelativeTransform` _returnvalue))
          (`PrimitiveComponent.SetMaterial` _returnvalue_5 0 "/Game/Tools/Hose/HoseMaterial_Inst.HoseMaterial_Inst")
          (`KismetArrayLibrary.Array_Add` (`self.AllSplineMeshes`) _returnvalue_5)
          (set `local.CurSplineMesh` _returnvalue_5)
          (`SplineMeshComponent.SetEndScale` _cursplinemesh _scalehose false)
          (`SplineMeshComponent.SetStartScale` _cursplinemesh _scalehose false)))
      (bind _returnvalue_6 (`KismetMathLibrary.InverseTransformLocation` (`self.GetTransform`) (`|GetArrayItem` _locations _output_get)))
      (bind _returnvalue_7 (- _returnvalue_6 _returnvalue_3))
      (bind _returnvalue_8 (* (select `bool` (== (`self.IndexAddWithSplineMeshSkip` _index 1) _returnvalue_2) :`false` (- (`KismetMathLibrary.InverseTransformLocation` (`self.GetTransform`) (`|GetArrayItem` _locations (`KismetMathLibrary.Round` (`KismetMathLibrary.Lerp` (`KismetMathLibrary.Conv_IntToDouble` (`local.CurNextIndex`)) (`KismetMathLibrary.Conv_IntToDouble` (`self.IndexAddWithSplineMeshSkip` _index 2)) (`self.TangentSampleFactor`))))) _returnvalue_3) :`true` (* (`SceneComponent.GetForwardVector` (`self.CurAttachEndCompoent`)) (`KismetMathLibrary.VSize` _returnvalue_7))) _tangentlengthfactor))
      (`SplineMeshComponent.SetStartAndEnd` _cursplinemesh (`KismetMathLibrary.SelectVector` _returnvalue_6 (stale _output_get_4) (== _output_get 0)) (`KismetMathLibrary.SelectVector` (* (select `bool` (== (`local.CurIndex`) 0) :`false` (- _returnvalue_6 (`KismetMathLibrary.InverseTransformLocation` (`self.GetTransform`) (`|GetArrayItem` _locations (`self.IndexAddWithSplineMeshSkip` _index -1 true)))) :`true` (* (`SceneComponent.GetForwardVector` (`self.Start`)) (`KismetMathLibrary.VSize` _returnvalue_7))) _tangentlengthfactor) (stale _output_get_3) (== (`local.CurIndex`) 0)) _returnvalue_4 _returnvalue_8 true)
      (bind _output_get_3 (set `local.LastEndTangent` _returnvalue_8))
      (bind _output_get_4 (set `local.LastPosition` _returnvalue_4)))))

(fn `UserConstructionScript`
  (bind _defaultattachendtocomponent (`self.DefaultAttachEndToComponent`))
  (bind _allsplinemeshes (`self.AllSplineMeshes`))
  (`ActorComponent.K2_DestroyComponent` _allsplinemeshes)
  (`KismetArrayLibrary.Array_Clear` _allsplinemeshes)
  (`CableComponent.SetAttachEndToComponent` (`self.Cable`) _defaultattachendtocomponent "None")
  (set `self.CurAttachEndCompoent` _defaultattachendtocomponent))