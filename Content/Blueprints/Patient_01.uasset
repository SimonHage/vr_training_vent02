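; Patient actor for a VR intubation training sequence, guiding the player from neck extension to connecting the ventilator.
; Starting an interaction on early steps loads a paused patient animation that interaction progress scrubs by position.
; Later steps destroy spawned laryngoscope or pouch actors by component-name match.
; StepComplete sets German instructions on the MotionControllerPawn and triggers the next step's ghost hint; a Debugging flag derives that step from CurrentStep.
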(event `self.InteractionStarted`
  (params (Step :type Integer))
  (bind _patient_maya_04_animation_01 (`self.Patient_Maya_04_animation_01`))
  (bind _patient_maya_04_animation_01_2 (`self.Patient_Maya_04_animation_01`))
  (bind _patient_maya_04_animation_01_3 (`self.Patient_Maya_04_animation_01`))
  (bind _patient_maya_04_animation_01_4 (`self.Patient_Maya_04_animation_01`))
  (`KismetSystemLibrary.PrintString` (`KismetStringLibrary.Concat_StrStr` "Interaction Started" (`KismetStringLibrary.Conv_IntToString` Step)))
  (bind _output_get (set `self.CurrentStep` Step))
  (switch `int` _output_get :!label _label
    (:`Default`
      (`SkeletalMeshComponent.PlayAnimation` _patient_maya_04_animation_01_3 "/Game/Animation/Patient_animation_01_mitZaehne.Patient_animation_01_mitZaehne" false)
      (`SkeletalMeshComponent.SetPosition` _patient_maya_04_animation_01_3 0.01 true)
      (`SkeletalMeshComponent.SetPlayRate` _patient_maya_04_animation_01_3 0.0))
    (:`0`
      (`SkeletalMeshComponent.PlayAnimation` _patient_maya_04_animation_01_4 "/Game/Animation/Patient_animation_01_mitZaehne.Patient_animation_01_mitZaehne" false)
      (`SkeletalMeshComponent.SetPosition` _patient_maya_04_animation_01_4 0.01 true)
      (`SkeletalMeshComponent.SetPlayRate` _patient_maya_04_animation_01_4 0.0)
      (set `self.ProgressCurrentStep` 0.01))
    (:`1`
      (`SkeletalMeshComponent.PlayAnimation` _patient_maya_04_animation_01 "/Game/Animation/Patient_animation_02_mitZaehne_Anim.Patient_animation_02_mitZaehne_Anim" false)
      (`SkeletalMeshComponent.SetPosition` _patient_maya_04_animation_01 0.01 true)
      (`SkeletalMeshComponent.SetPlayRate` _patient_maya_04_animation_01 0.0)
      (set `self.ProgressCurrentStep` 0.01))
    (:`2`
      (`SkeletalMeshComponent.PlayAnimation` _patient_maya_04_animation_01_2 "/Game/Animation/Patient_animation_03_mitZaehne_Anim.Patient_animation_03_mitZaehne_Anim" false)
      (`SkeletalMeshComponent.SetPosition` _patient_maya_04_animation_01_2 0.01 true)
      (`SkeletalMeshComponent.SetPlayRate` _patient_maya_04_animation_01_2 0.0)
      (set `self.ProgressCurrentStep` 0.01))
    (:`4`
      (for _array_element (`self.SpawnedActors`)
        (bind _asstatic_mesh_actor (cast `StaticMeshActor` _array_element))
        (if (>= (`KismetStringLibrary.FindSubstring` (`KismetSystemLibrary.GetDisplayName` (`StaticMeshActor.StaticMeshComponent` _asstatic_mesh_actor)) "laryn") 0)
          (`self.K2_DestroyActor` _array_element))))
    (:`8`
      (for _array_element_2 (`self.SpawnedActors`)
        (bind _asskeletal_mesh_actor (cast `SkeletalMeshActor` _array_element_2))
        (if (>= (`KismetStringLibrary.FindSubstring` (`KismetSystemLibrary.GetDisplayName` (`SkeletalMeshActor.SkeletalMeshComponent` _asskeletal_mesh_actor)) "pouch") 0)
          (`self.K2_DestroyActor` _array_element_2))))))

(event `self.Interacting`
  (params (Progress :type "Float (single-precision)"))
  (switch `int` (`self.CurrentStep`)
    (:`0`
      (bind _output_get (set `self.ProgressCurrentStep` Progress))
      (`SkeletalMeshComponent.SetPosition` (`self.Patient_Maya_04_animation_01`) _output_get true))
    (:`1`
      (bind _output_get_2 (set `self.ProgressCurrentStep` Progress))
      (`SkeletalMeshComponent.SetPosition` (`self.Patient_Maya_04_animation_01`) _output_get_2 true))
    (:`2`
      (bind _output_get_3 (set `self.ProgressCurrentStep` Progress))
      (`SkeletalMeshComponent.SetPosition` (`self.Patient_Maya_04_animation_01`) _output_get_3 true))))

(event `self.ReceiveBeginPlay`
  (`|ExecutionSequence`
    (:`then_0`
      (goto _label))
    (:`then_1`
      (if (`self.Debugging`)
        (switch `int` (stale `self.StepComplete` _output_get) :!label _label_2
          (:`Default`
            (message `/Game/Blueprints/TrainingStepInterface.StartGhost` (`|GetArrayItem` (`self.StepArray`)) :!label _label_3)
            (message `/Game/Blueprints/TrainingStepInterface.StartGhost` (`|GetArrayItem` (`self.StepArray`) 1))
            (bind _asmotion_controller_pawn (cast `/Game/VirtualRealityBP/Blueprints/MotionControllerPawn` (`GameplayStatics.GetPlayerPawn` 0)))
            (`TextRenderComponent.K2_SetText` (`/Game/VirtualRealityBP/Blueprints/MotionControllerPawn.SchrittText` _asmotion_controller_pawn) "Schritt 1:")
            (`TextRenderComponent.K2_SetText` (`/Game/VirtualRealityBP/Blueprints/MotionControllerPawn.AnweisungsText` _asmotion_controller_pawn) "Bitte nun den Nacken \ndes Patienten über- \nstrecken"))
          (:`0`
            (bind _asmotion_controller_pawn_2 (cast `/Game/VirtualRealityBP/Blueprints/MotionControllerPawn` (`GameplayStatics.GetPlayerPawn` 0)))
            (`TextRenderComponent.K2_SetText` (`/Game/VirtualRealityBP/Blueprints/MotionControllerPawn.SchrittText` _asmotion_controller_pawn_2) "Schritt 2:")
            (`TextRenderComponent.K2_SetText` (`/Game/VirtualRealityBP/Blueprints/MotionControllerPawn.AnweisungsText` _asmotion_controller_pawn_2) "Bitte öffnen Sie \nden Mund des \nPatienten")
            (`KismetSystemLibrary.Delay` 2.0)
            (message `/Game/Blueprints/TrainingStepInterface.StartGhost` (`|GetArrayItem` (`self.StepArray`) 2)))
          (:`1`
            (bind _asmotion_controller_pawn_3 (cast `/Game/VirtualRealityBP/Blueprints/MotionControllerPawn` (`GameplayStatics.GetPlayerPawn` 0)))
            (`TextRenderComponent.K2_SetText` (`/Game/VirtualRealityBP/Blueprints/MotionControllerPawn.SchrittText` _asmotion_controller_pawn_3) "Schritt 3:")
            (`TextRenderComponent.K2_SetText` (`/Game/VirtualRealityBP/Blueprints/MotionControllerPawn.AnweisungsText` _asmotion_controller_pawn_3) "Bitte führen Sie das \nLaryngoskop am rechten \nMundwinkel ein. \nWeiterführung nach links.")
            (`KismetSystemLibrary.Delay` 2.0)
            (message `/Game/Blueprints/TrainingStepInterface.StartGhost` (`|GetArrayItem` (`self.StepArray`) 3)))
          (:`2`
            (bind _asmotion_controller_pawn_4 (cast `/Game/VirtualRealityBP/Blueprints/MotionControllerPawn` (`GameplayStatics.GetPlayerPawn` 0)))
            (`TextRenderComponent.K2_SetText` (`/Game/VirtualRealityBP/Blueprints/MotionControllerPawn.SchrittText` _asmotion_controller_pawn_4) "Schritt 4:")
            (`TextRenderComponent.K2_SetText` (`/Game/VirtualRealityBP/Blueprints/MotionControllerPawn.AnweisungsText` _asmotion_controller_pawn_4) "Bitte führen Sie den \nTubus bis zur Markierung ein.")
            (`KismetSystemLibrary.Delay` 2.0)
            (message `/Game/Blueprints/TrainingStepInterface.StartGhost` (`|GetArrayItem` (`self.StepArray`) 4)))
          (:`3`
            (bind _asmotion_controller_pawn_5 (cast `/Game/VirtualRealityBP/Blueprints/MotionControllerPawn` (`GameplayStatics.GetPlayerPawn` 0)))
            (`TextRenderComponent.K2_SetText` (`/Game/VirtualRealityBP/Blueprints/MotionControllerPawn.SchrittText` _asmotion_controller_pawn_5) "Schritt 5:")
            (`TextRenderComponent.K2_SetText` (`/Game/VirtualRealityBP/Blueprints/MotionControllerPawn.AnweisungsText` _asmotion_controller_pawn_5) "Laryngoskop entfernen..")
            (`KismetSystemLibrary.Delay` 2.0)
            (message `/Game/Blueprints/TrainingStepInterface.StartGhost` (`|GetArrayItem` (`self.StepArray`) 5)))
          (:`4`
            (bind _asmotion_controller_pawn_6 (cast `/Game/VirtualRealityBP/Blueprints/MotionControllerPawn` (`GameplayStatics.GetPlayerPawn` 0)))
            (`TextRenderComponent.K2_SetText` (`/Game/VirtualRealityBP/Blueprints/MotionControllerPawn.SchrittText` _asmotion_controller_pawn_6) "Schritt 6:")
            (`TextRenderComponent.K2_SetText` (`/Game/VirtualRealityBP/Blueprints/MotionControllerPawn.AnweisungsText` _asmotion_controller_pawn_6) "Bitte den Tubus mithilfe der  \nBlockerspritze fixieren.")
            (`KismetSystemLibrary.Delay` 2.0)
            (message `/Game/Blueprints/TrainingStepInterface.StartGhost` (`|GetArrayItem` (`self.StepArray`) 6)))
          (:`5`
            (bind _asmotion_controller_pawn_7 (cast `/Game/VirtualRealityBP/Blueprints/MotionControllerPawn` (`GameplayStatics.GetPlayerPawn` 0)))
            (`TextRenderComponent.K2_SetText` (`/Game/VirtualRealityBP/Blueprints/MotionControllerPawn.SchrittText` _asmotion_controller_pawn_7) "Schritt 7:")
            (`TextRenderComponent.K2_SetText` (`/Game/VirtualRealityBP/Blueprints/MotionControllerPawn.AnweisungsText` _asmotion_controller_pawn_7) "Nun den Ambubeutel am Tubus \nanschließen.")
            (`KismetSystemLibrary.Delay` 2.0)
            (message `/Game/Blueprints/TrainingStepInterface.StartGhost` (`|GetArrayItem` (`self.StepArray`) 7)))
          (:`6`
            (bind _asmotion_controller_pawn_8 (cast `/Game/VirtualRealityBP/Blueprints/MotionControllerPawn` (`GameplayStatics.GetPlayerPawn` 0)))
            (`TextRenderComponent.K2_SetText` (`/Game/VirtualRealityBP/Blueprints/MotionControllerPawn.SchrittText` _asmotion_controller_pawn_8) "Schritt 7:")
            (`TextRenderComponent.K2_SetText` (`/Game/VirtualRealityBP/Blueprints/MotionControllerPawn.AnweisungsText` _asmotion_controller_pawn_8) "Mithilfe des Ambubeutels die \nBeatmungsfunktion kontrollieren.")
            (`KismetSystemLibrary.Delay` 2.0)
            (message `/Game/Blueprints/TrainingStepInterface.StartGhost` (`|GetArrayItem` (`self.StepArray`) 8)))
          (:`7`
            (bind _asmotion_controller_pawn_9 (cast `/Game/VirtualRealityBP/Blueprints/MotionControllerPawn` (`GameplayStatics.GetPlayerPawn` 0)))
            (`TextRenderComponent.K2_SetText` (`/Game/VirtualRealityBP/Blueprints/MotionControllerPawn.SchrittText` _asmotion_controller_pawn_9) "Schritt 8:")
            (`TextRenderComponent.K2_SetText` (`/Game/VirtualRealityBP/Blueprints/MotionControllerPawn.AnweisungsText` _asmotion_controller_pawn_9) "Nun das Beatmungsgerät an den  \nTubus anschließen.")
            (`KismetSystemLibrary.Delay` 2.0)
            (message `/Game/Blueprints/TrainingStepInterface.StartGhost` (`|GetArrayItem` (`self.StepArray`) 9)))
          (:`8`
            (bind _asmotion_controller_pawn_10 (cast `/Game/VirtualRealityBP/Blueprints/MotionControllerPawn` (`GameplayStatics.GetPlayerPawn` 0)))
            (`TextRenderComponent.K2_SetText` (`/Game/VirtualRealityBP/Blueprints/MotionControllerPawn.SchrittText` _asmotion_controller_pawn_10) "")
            (`TextRenderComponent.K2_SetText` (`/Game/VirtualRealityBP/Blueprints/MotionControllerPawn.AnweisungsText` _asmotion_controller_pawn_10) "")))
        (else
          (goto _label_3))))))

(event `self.StepComplete`
  (params (Step :type Integer))
  (bind _output_get (set `self.StepToset` (`KismetMathLibrary.SelectInt` (- (`self.CurrentStep`) 1) Step (`self.Debugging`))))
  (goto _label_2))

(fn `UserConstructionScript`)