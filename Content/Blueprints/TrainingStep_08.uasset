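; Training step 8 actor: a ghost hand demonstrates a pouch action on the patient for the player to take over.
; Until grabbed, Tick loops the hand offset and pouch morph as a preview.
; Pickup by the matching controller swaps materials, hides the player's hand and advances both by hold time, not controller motion, feeding progress to Patient_01.
; Completion notifies the patient, then releases and destroys all instances of this step.
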(event `/Game/Blueprints/TrainingStepInterface.StartGhost`
  (`self.SetActorHiddenInGame` false)
  (`self.SetActorEnableCollision` true)
  (`PrimitiveComponent.SetCollisionEnabled` (select `bool` (`self.Right`) :`false` (`self.Sphere1`) :`true` (`self.Sphere`)) "QueryAndPhysics")
  (`self.SetActorTickEnabled` true))

(event `self.ReceiveBeginPlay`
  (bind _outactors (`GameplayStatics.GetAllActorsOfClass` "/Game/Blueprints/TrainingStepManager.TrainingStepManager_C"))
  (set `self.TrainingStepManager` (`|GetArrayItem` _outactors))
  (bind _outactors_2 (`GameplayStatics.GetAllActorsOfClass` "/Game/Blueprints/Patient_01.Patient_01_C"))
  (set `self.Patient` (`|GetArrayItem` _outactors_2))
  (if (`self.Right`)
    (set `self.StartTransfHand` (`SceneComponent.K2_GetComponentToWorld` (`self.Hand_01_R`)))
    (else
      (set `self.StartTransfHand` (`SceneComponent.K2_GetComponentToWorld` (`self.Hand_02_L`))))))

(event `/Game/VirtualRealityBP/Blueprints/PickupActorInterface.Pickup`
  (params (AttachTo :type "SceneComponent Object Reference") (BP_Controller :type "/Game/VirtualRealityBP/Blueprints/BP_MotionController Object Reference"))
  (bind _patient (`self.Patient`))
  (bind _step (`self.Step`))
  (bind _motioncontroller (`/Game/VirtualRealityBP/Blueprints/BP_MotionController.MotionController` (`self.GrabbingController`)))
  (if (and (`self.Right`) (`|EnumEquality` (`/Game/VirtualRealityBP/Blueprints/BP_MotionController.Hand` BP_Controller) "Right"))
    (`/Game/Blueprints/TrainingStepInterface.InteractionStarted` _patient _step)
    (set `self.GrabbingController` BP_Controller :!label _label)
    (`SceneComponent.SetVisibility` (`/Game/VirtualRealityBP/Blueprints/BP_MotionController.HandMesh` (`self.GrabbingController`)) false false)
    (if (`self.Right`)
      (`PrimitiveComponent.SetMaterial` (`self.Hand_01_R`) 0 "/Game/VRHandPoses/UnrealVRHand/Mesh/GloveMat_Inst.GloveMat_Inst")
      (`PrimitiveComponent.SetMaterial` (`self.Pouch`) 0 "/Game/TexturesMats/PouchMat.PouchMat")
      (else
        (`PrimitiveComponent.SetMaterial` (`self.Hand_02_L`) 0 "/Game/VRHandPoses/UnrealVRHand/Mesh/GloveMat_Inst.GloveMat_Inst")))
    (set `self.InteractionRunning` true)
    (set `self.StartRotationController` (`SceneComponent.K2_GetComponentRotation` _motioncontroller))
    (set `self.StartLocationController` (`SceneComponent.K2_GetComponentLocation` _motioncontroller))
    (elif (and (`|EnumEquality` (`/Game/VirtualRealityBP/Blueprints/BP_MotionController.Hand` BP_Controller) "Left") (not (`self.Right`)))
      (`/Game/Blueprints/TrainingStepInterface.InteractionStarted` _patient _step)
      (goto _label))))

(event `/Game/VirtualRealityBP/Blueprints/PickupActorInterface.Drop`
  (`SceneComponent.SetVisibility` (`/Game/VirtualRealityBP/Blueprints/BP_MotionController.HandMesh` (`self.GrabbingController`)) true false)
  (if (`self.Right`)
    (`PrimitiveComponent.SetMaterial` (`self.Hand_01_R`) 0 "/Game/VRHandPoses/UnrealVRHand/Mesh/GloveMatGhost.GloveMatGhost")
    (else
      (`PrimitiveComponent.SetMaterial` (`self.Hand_02_L`) 0 "/Game/VRHandPoses/UnrealVRHand/Mesh/GloveMatGhost.GloveMatGhost")))
  (set `self.InteractionRunning` false))

(event `StepFinished`
  (`SceneComponent.SetVisibility` (`/Game/VirtualRealityBP/Blueprints/BP_MotionController.HandMesh` (`self.GrabbingController`)) true false)
  (`/Game/VirtualRealityBP/Blueprints/BP_MotionController.ReleaseActor` (`self.GrabbingController`))
  (`self.K2_DestroyActor`))

(event `self.ReceiveTick`
  (params (DeltaSeconds :type "Float (single-precision)"))
  (bind _ghostanim (`self.GhostAnim`))
  (bind (_handendtransf_location _handendtransf_rotation _handendtransf_scale) (`KismetMathLibrary.BreakTransform` (`self.HandEndTransf`)))
  (bind (_handendtransf_location_2 _handendtransf_rotation_2 _handendtransf_scale_2) (`KismetMathLibrary.BreakTransform` (`self.HandEndTransf`)))
  (bind (_handendtransf_location_3 _handendtransf_rotation_3 _handendtransf_scale_3) (`KismetMathLibrary.BreakTransform` (`self.HandEndTransf`)))
  (bind (_handendtransf_location_4 _handendtransf_rotation_4 _handendtransf_scale_4) (`KismetMathLibrary.BreakTransform` (`self.HandEndTransf`)))
  (bind _starttransfhand (`self.StartTransfHand`))
  (bind _starttransfhand_2 (`self.StartTransfHand`))
  (`self.UpdateHandMEsh`)
  (if (`self.StepCompleted`)
    _
    (elif (`self.InteractionRunning`)
      (`self.UpdateHandMEsh`)
      (bind _output_get (set `self.Timer` (+ (`self.Timer`) (/ (`GameplayStatics.GetWorldDeltaSeconds`) (`self.GhostAnimSec`)))))
      (bind _returnvalue (`KismetMathLibrary.FClamp` _output_get 0.01))
      (`/Game/Blueprints/Patient_01.Interacting` (`self.Patient`) _returnvalue)
      (if (`self.Right`)
        (`self.MeshOffset` _returnvalue (`self.Hand_01_R`) _starttransfhand_2 (`KismetMathLibrary.MakeTransform` _handendtransf_location_4 _handendtransf_rotation_4 _handendtransf_scale_4))
        (else
          (`self.MeshOffset` _returnvalue (`self.Hand_02_L`) _starttransfhand_2 (`KismetMathLibrary.MakeTransform` _handendtransf_location_3 _handendtransf_rotation_3 _handendtransf_scale_3))))
      (`SkeletalMeshComponent.SetMorphTarget` (`self.Pouch`) "Key 1" _returnvalue true)
      (if (>= _returnvalue 1.0)
        (set `self.StepCompleted` true)
        (`/Game/Blueprints/Patient_01.StepComplete` (`self.Patient`) (`self.Step`))
        (bind _outactors (`GameplayStatics.GetAllActorsOfClass` "TrainingStep_08_C"))
        (for _array_element _outactors
          (`self.StepFinished` _array_element)))
      (else
        (if (`self.Right`)
          (`self.MeshOffset` _ghostanim (`self.Hand_01_R`) _starttransfhand (`KismetMathLibrary.MakeTransform` _handendtransf_location_2 _handendtransf_rotation_2 _handendtransf_scale_2))
          (else
            (`self.MeshOffset` _ghostanim (`self.Hand_02_L`) _starttransfhand (`KismetMathLibrary.MakeTransform` _handendtransf_location _handendtransf_rotation _handendtransf_scale))))
        (bind _output_get_2 (set `self.GhostAnim` (+ (`self.GhostAnim`) (/ (`GameplayStatics.GetWorldDeltaSeconds`) (`self.GhostAnimSec`)))))
        (`SkeletalMeshComponent.SetMorphTarget` (`self.Pouch`) "Key 1" _output_get_2 false)
        (if (>= _output_get_2 1.0)
          (set `self.GhostAnim` 0.0))))))

(event `UpdateHandMEsh`
  (if (`self.Right`)
    (bind _asmannequin_hand_right_anim_bp (cast `/Game/VRHandPoses/UnrealVRHand/Mesh/MannequinHand_Right_AnimBP` (`SkeletalMeshComponent.GetAnimInstance` (`self.Hand_01_R`))))
    (`/Game/VRHandPoses/UnrealVRHand/Mesh/MannequinHand_Right_AnimBP.SetPose` _asmannequin_hand_right_anim_bp (`self.GripState`) (`self.CurSpecificGrabType`) true true)
    (`/Engine/EditorBlueprintResources/StandardMacros.Gate` false
      (:`Exit`
        (set `/Game/VRHandPoses/UnrealVRHand/Mesh/MannequinHand_Right_AnimBP.CurGrabDebugOverwrite-ForceGrabInEditor` true _asmannequin_hand_right_anim_bp)))
    (else
      (bind _asmannequin_hand_right_anim_bp_2 (cast `/Game/VRHandPoses/UnrealVRHand/Mesh/MannequinHand_Right_AnimBP` (`SkeletalMeshComponent.GetAnimInstance` (`self.Hand_02_L`))))
      (`/Game/VRHandPoses/UnrealVRHand/Mesh/MannequinHand_Right_AnimBP.SetPose` _asmannequin_hand_right_anim_bp_2 (`self.GripState`) (`self.CurSpecificGrabType`) true true)
      (`/Engine/EditorBlueprintResources/StandardMacros.Gate` false
        (:`Exit`
          (set `/Game/VRHandPoses/UnrealVRHand/Mesh/MannequinHand_Right_AnimBP.CurGrabDebugOverwrite-ForceGrabInEditor` true _asmannequin_hand_right_anim_bp_2))))))

(fn `MeshOffset`
  (params (AnimationsProgress :type "Float (double-precision)") (Mesh :type "SceneComponent Object Reference") (StartTransform :type "Transform Structure") (TransformDiff :type "Transform Structure"))
  (`SceneComponent.K2_SetWorldTransform` Mesh (`KismetMathLibrary.MakeTransform` (+ (.location StartTransform) (* TransformDiff_Location AnimationsProgress)) (`KismetMathLibrary.MakeRotator` (+ (* (.roll (.rotation TransformDiff)) AnimationsProgress) (.roll (.rotation StartTransform))) (+ (* (.pitch (.rotation TransformDiff)) AnimationsProgress) (.pitch (.rotation StartTransform))) (+ (* (.yaw (.rotation TransformDiff)) AnimationsProgress) (.yaw (.rotation StartTransform)))) (.scale StartTransform)) false false))

(fn `UserConstructionScript`
  (bind _hand_02_l (`self.Hand_02_L`))
  (bind _hand_01_r (`self.Hand_01_R`))
  (if (not (`self.Both`))
    (if (`self.Right`)
      (for _array_element (`SceneComponent.GetChildrenComponents` _hand_02_l true)
        (`ActorComponent.K2_DestroyComponent` _array_element))
      (`ActorComponent.K2_DestroyComponent` _hand_02_l)
      (else
        (for _array_element_2 (`SceneComponent.GetChildrenComponents` _hand_01_r true)
          (`ActorComponent.K2_DestroyComponent` _array_element_2))
        (`ActorComponent.K2_DestroyComponent` _hand_01_r)))
    (`self.UpdateHandMEsh`)))