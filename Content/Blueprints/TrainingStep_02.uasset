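; VR training step showing a left or right ghost glove hand that loops a demonstration motion on a patient.
; Pickup by the matching controller hides its hand, makes the glove solid and starts the Patient_01 interaction.
; Tick turns controller pitch and X movement since pickup into clamped progress, driving both the patient and the glove's transform offset.
; Full progress completes the patient's step, then releases and destroys every TrainingStep_02 instance.
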(event `/Game/Blueprints/TrainingStepInterface.StartGhost`
  (bind _sphere (`self.Sphere`))
  (`self.SetActorHiddenInGame` false)
  (`self.SetActorEnableCollision` true)
  (`PrimitiveComponent.SetCollisionEnabled` (select `bool` (`KismetSystemLibrary.IsValid` _sphere) :`false` (`self.Sphere1`) :`true` _sphere) "QueryAndPhysics"))

(event `self.ReceiveBeginPlay`
  (bind _outactors (`GameplayStatics.GetAllActorsOfClass` "/Game/Blueprints/TrainingStepManager.TrainingStepManager_C"))
  (set `self.TrainingStepManager` (`|GetArrayItem` _outactors))
  (bind _outactors_2 (`GameplayStatics.GetAllActorsOfClass` "/Game/Blueprints/Patient_01.Patient_01_C"))
  (set `self.Patient` (`|GetArrayItem` _outactors_2))
  (if (`self.Right`)
    (set `self.StartTransfHand` (`SceneComponent.K2_GetComponentToWorld` (`self.Hand_01_R`)))
    (else
      (set `self.StartTransfHand` (`SceneComponent.K2_GetComponentToWorld` (`self.Hand_02_L`)))))
  (`self.UpdateHandMEsh`))

(event `/Game/VirtualRealityBP/Blueprints/PickupActorInterface.Pickup`
  (params (AttachTo :type "SceneComponent Object Reference") (BP_Controller :type "/Game/VirtualRealityBP/Blueprints/BP_MotionController Object Reference"))
  (bind _patient (`self.Patient`))
  (bind _grabbingcontroller (`self.GrabbingController`))
  (bind _step (`self.Step`))
  (if (and (`self.Right`) (`|EnumEquality` (`/Game/VirtualRealityBP/Blueprints/BP_MotionController.Hand` BP_Controller) "Right"))
    (`/Game/Blueprints/TrainingStepInterface.InteractionStarted` _patient _step)
    (set `self.GrabbingController` BP_Controller :!label _label)
    (`SceneComponent.SetVisibility` (`/Game/VirtualRealityBP/Blueprints/BP_MotionController.HandMesh` (`self.GrabbingController`)) false false)
    (if (`self.Right`)
      (`PrimitiveComponent.SetMaterial` (`self.Hand_01_R`) 0 "/Game/VRHandPoses/UnrealVRHand/Mesh/GloveMat_Inst.GloveMat_Inst")
      (else
        (`PrimitiveComponent.SetMaterial` (`self.Hand_02_L`) 0 "/Game/VRHandPoses/UnrealVRHand/Mesh/GloveMat_Inst.GloveMat_Inst")))
    (set `self.InteractionRunning` true)
    (set `self.StartRotationController` (`SceneComponent.K2_GetComponentRotation` (`/Game/VirtualRealityBP/Blueprints/BP_MotionController.MotionController` _grabbingcontroller)))
    (set `self.StartLocationController` (`SceneComponent.K2_GetComponentLocation` (`/Game/VirtualRealityBP/Blueprints/BP_MotionController.MotionController` _grabbingcontroller)))
    (elif (and (`|EnumEquality` (`/Game/VirtualRealityBP/Blueprints/BP_MotionController.Hand` BP_Controller) "Left") (not (`self.Right`)))
      (`/Game/Blueprints/TrainingStepInterface.InteractionStarted` _patient _step)
      (goto _label))))

(event `/Game/VirtualRealityBP/Blueprints/PickupActorInterface.Drop`
  (`SceneComponent.SetVisibility` (`/Game/VirtualRealityBP/Blueprints/BP_MotionController.HandMesh` (`self.GrabbingController`)) true false)
  (if (`self.Right`)
    (`PrimitiveComponent.SetMaterial` (`self.Hand_01_R`) 0 "/Game/VRHandPoses/UnrealVRHand/Mesh/GloveMatGhost.GloveMatGhost")
    (else
      (`PrimitiveComponent.SetMaterial` (`self.Hand_02_L`) 0 "/Game/VRHandPoses/UnrealVRHand/Mesh/GloveMatGhost.GloveMatGhost")))
  (set `self.InteractionRunning` false))

(event `StepFinished`
  (`SceneComponent.SetVisibility` (`/Game/VirtualRealityBP/Blueprints/BP_MotionController.HandMesh` (`self.GrabbingController`)) true false)
  (`/Game/VirtualRealityBP/Blueprints/BP_MotionController.ReleaseActor` (`self.GrabbingController`))
  (`self.K2_DestroyActor`))

(event `self.ReceiveTick`
  (params (DeltaSeconds :type "Float (single-precision)"))
  (bind _ghostanim (`self.GhostAnim`))
  (bind (_startrotationcontroller_roll _startrotationcontroller_pitch) (`KismetMathLibrary.BreakRotator` (`self.StartRotationController`)))
  (bind _startlocationcontroller_x (`KismetMathLibrary.BreakVector` (`self.StartLocationController`)))
  (bind (_returnvalue_roll _returnvalue_pitch) (`KismetMathLibrary.BreakRotator` (`SceneComponent.K2_GetComponentRotation` (`/Game/VirtualRealityBP/Blueprints/BP_MotionController.MotionController` (`self.GrabbingController`)))))
  (bind _returnvalue_x (`KismetMathLibrary.BreakVector` (`SceneComponent.K2_GetComponentLocation` (`/Game/VirtualRealityBP/Blueprints/BP_MotionController.MotionController` (`self.GrabbingController`)))))
  (bind _returnvalue (`KismetMathLibrary.FClamp` (+ (/ (- _startrotationcontroller_pitch _returnvalue_pitch) 25.0) (/ (- _returnvalue_x _startlocationcontroller_x) 15.0)) 0.1))
  (`self.UpdateHandMEsh`)
  (if (`self.StepCompleted`)
    _
    (elif (`self.InteractionRunning`)
      (`/Game/Blueprints/Patient_01.Interacting` (`self.Patient`) _returnvalue)
      (if (`self.Right`)
        (`self.HandOffset` _returnvalue (`self.HandEndTransf`) (`self.Hand_01_R`))
        (else
          (`self.HandOffset` _returnvalue (`self.HandEndTransf`) (`self.Hand_02_L`))))
      (if (>= _returnvalue 1.0)
        (set `self.StepCompleted` true)
        (`/Game/Blueprints/Patient_01.StepComplete` (`self.Patient`) (`self.Step`))
        (bind _outactors (`GameplayStatics.GetAllActorsOfClass` "TrainingStep_02_C"))
        (for _array_element _outactors
          (`self.StepFinished` _array_element)))
      (else
        (if (`self.Right`)
          (`self.HandOffset` _ghostanim (`self.HandEndTransf`) (`self.Hand_01_R`))
          (else
            (`self.HandOffset` _ghostanim (`self.HandEndTransf`) (`self.Hand_02_L`))))
        (bind _output_get (set `self.GhostAnim` (+ (`self.GhostAnim`) (/ (`GameplayStatics.GetWorldDeltaSeconds`) (`self.GhostAnimSec`)))))
        (if (>= _output_get 1.0)
          (set `self.GhostAnim` 0.0))))))

(event `UpdateHandMEsh`
  (if (`self.Right`)
    (bind _asmannequin_hand_right_anim_bp (cast `/Game/VRHandPoses/UnrealVRHand/Mesh/MannequinHand_Right_AnimBP` (`SkeletalMeshComponent.GetAnimInstance` (`self.Hand_01_R`))))
    (`/Game/VRHandPoses/UnrealVRHand/Mesh/MannequinHand_Right_AnimBP.SetPose` _asmannequin_hand_right_anim_bp (`self.GripState`) (`self.CurSpecificGrabType`) true false)
    (`/Engine/EditorBlueprintResources/StandardMacros.Gate` false
      (:`Exit`
        (set `/Game/VRHandPoses/UnrealVRHand/Mesh/MannequinHand_Right_AnimBP.CurGrabDebugOverwrite-ForceGrabInEditor` true _asmannequin_hand_right_anim_bp)))
    (else
      (bind _asmannequin_hand_right_anim_bp_2 (cast `/Game/VRHandPoses/UnrealVRHand/Mesh/MannequinHand_Right_AnimBP` (`SkeletalMeshComponent.GetAnimInstance` (`self.Hand_02_L`))))
      (`/Game/VRHandPoses/UnrealVRHand/Mesh/MannequinHand_Right_AnimBP.SetPose` _asmannequin_hand_right_anim_bp_2 (`self.GripState`) (`self.CurSpecificGrabType`) true false)
      (`/Engine/EditorBlueprintResources/StandardMacros.Gate` false
        (:`Exit`
          (set `/Game/VRHandPoses/UnrealVRHand/Mesh/MannequinHand_Right_AnimBP.CurGrabDebugOverwrite-ForceGrabInEditor` true _asmannequin_hand_right_anim_bp_2))))))

(fn `HandOffset`
  (params (AnimationsProgress :type "Float (double-precision)") (TransformDiff :type "Transform Structure") (Mesh :type "SceneComponent Object Reference"))
  (bind _starttransfhand (`self.StartTransfHand`))
  (`SceneComponent.K2_SetWorldTransform` Mesh (`KismetMathLibrary.MakeTransform` (+ (.location _starttransfhand) (* TransformDiff_Location AnimationsProgress)) (`KismetMathLibrary.MakeRotator` (+ (* (.roll (.rotation TransformDiff)) AnimationsProgress) (.roll (.rotation _starttransfhand))) (+ (* (.pitch (.rotation TransformDiff)) AnimationsProgress) (.pitch (.rotation _starttransfhand))) (+ (* (.yaw (.rotation TransformDiff)) AnimationsProgress) (.yaw (.rotation _starttransfhand)))) (.scale _starttransfhand)) false false))

(fn `UserConstructionScript`
  (bind _hand_01_r (`self.Hand_01_R`))
  (bind _hand_02_l (`self.Hand_02_L`))
  (if (not (`self.Both`))
    (if (`self.Right`)
      (for _array_element (`SceneComponent.GetChildrenComponents` _hand_02_l true)
        (`ActorComponent.K2_DestroyComponent` _array_element))
      (`ActorComponent.K2_DestroyComponent` _hand_02_l)
      (else
        (for _array_element_2 (`SceneComponent.GetChildrenComponents` _hand_01_r true)
          (`ActorComponent.K2_DestroyComponent` _array_element_2))
        (`ActorComponent.K2_DestroyComponent` _hand_01_r)))
    (`self.UpdateHandMEsh`)))